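; BP_Flyer is a flying enemy that shoots projectiles at the player.
; Tick swaps its material by player 2D distance and, through a three-second Delay, turns it to face the player and fires with velocity-based lead aiming at any range.
; Capsule overlap damages the player; pistol bullets hitting the Box destroy both.
; A delayed respawn follows DestroyActor in the same chain, and a separate Respawn event is never called here.
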(event OnComponentBeginOverlap(CapsuleComponent)
  (params (OverlappedComponent :type Primitive%20Component%20Object%20Reference) (OtherActor :type Actor%20Object%20Reference) (OtherComp :type Primitive%20Component%20Object%20Reference) (OtherBodyIndex :type Integer) (bFromSweep :type Boolean) (SweepResult :type Hit%20Result%20Structure%20%28by%20ref%29))
  (Utilities|Casting|CastToHorrorEngineCharacter OtherActor)
  (bind _asmaster (CallFunction|GetPlayer))
  (Default|GetDamage :self _asmaster :DamagePoint 1e+01))

(event OnComponentBeginOverlap(Box)
  (params (OverlappedComponent :type Primitive%20Component%20Object%20Reference) (OtherActor :type Actor%20Object%20Reference) (OtherComp :type Primitive%20Component%20Object%20Reference) (OtherBodyIndex :type Integer) (bFromSweep :type Boolean) (SweepResult :type Hit%20Result%20Structure%20%28by%20ref%29))
  (bind _aspistol_bullets (Utilities|Casting|CastToPistolBullets OtherActor)
    (:then
      _)
    (:CastFailed
      (bind _aspistol_bullet_bp (Utilities|Casting|CastToPistolBullet_BP OtherActor))))
  (Actor|DestroyActor _aspistol_bullets)
  (Actor|DestroyActor)
  (Development|PrintString "Hello")
  (Utilities|FlowControl|Delay 7.0)
  (Development|PrintString "done")
  (Game|SpawnActorfromClass "BP_Flyer_C" (Math|Transform|MakeTransform (Transformation|GetActorLocation) "0, 0, 0" "1.000000,1.000000,1.000000") "Undefined" 0 0))

(event Custom|Respawn
  (Utilities|FlowControl|Delay 1e+01)
  (Game|SpawnActorfromClass "BP_Flyer_C" (Math|Transform|MakeTransform (Transformation|GetActorLocation) "0, 0, 0" "1.000000,1.000000,1.000000") "Undefined" 0 0))

(event EventBeginPlay
  (bind _ashorror_engine_character (Utilities|Casting|CastToHorrorEngineCharacter (Game|GetPlayerCharacter 0)))
  (Variables|Default|SetPlayerRef _ashorror_engine_character))

(event EventTick
  (params (DeltaSeconds :type Float%20%28single-precision%29))
  (bind _returnvalue (Transformation|GetActorLocation))
  (bind _box (Variables|Default|GetBox))
  (bind _samplefigure (Variables|Default|GetSampleFigure))
  (bind _returnvalue_2 (Transformation|GetWorldLocation _box))
  (bind _ashorror_engine_character (Utilities|Casting|CastToHorrorEngineCharacter (Game|GetPlayerCharacter 0)))
  (if (<= (Math|Vector|Distance2D(Vector) (Math|Vector2D|MakeVector2D (.x (Transformation|GetActorLocation _ashorror_engine_character)) (.y (Transformation|GetActorLocation _ashorror_engine_character))) (Math|Vector2D|MakeVector2D (.x _returnvalue) (.y _returnvalue))) 2984.0)
    (Rendering|Material|SetMaterial _samplefigure 0 "/Engine/VREditor/LaserPointer/LaserPointerMaterial.LaserPointerMaterial")
    (else
      (Rendering|Material|SetMaterial _samplefigure 0 "/Game/HorrorEngine/Materials/He_Noise.He_Noise")))
  (Utilities|FlowControl|Delay 3.0)
  (bind _ashorror_engine_character_2 (Utilities|Casting|CastToHorrorEngineCharacter (Game|GetPlayerCharacter 0)))
  (Transformation|SetActorRotation (Math|Rotator|FindLookatRotation _returnvalue_2 (Transformation|GetWorldLocation (Variables|/Script/Engine.Actor|GetRootComponent _ashorror_engine_character_2))))
  (Game|SpawnActorfromClass "/Game/HorrorEngine/Blueprints/Enemy/EnemyProjectile.EnemyProjectile_C" (Math|Transform|MakeTransform _returnvalue_2 (Math|Rotator|FindLookatRotation _returnvalue_2 (+ (Transformation|GetWorldLocation (Variables|/Script/Engine.Actor|GetRootComponent _ashorror_engine_character_2)) (* (Transformation|GetVelocity _ashorror_engine_character_2) (/ (Transformation|GetDistanceTo _ashorror_engine_character_2) 1e+03))))) "Undefined" 0 0))

(fn ConstructionScript)

(fn UpdateFlySpeed
  (params (New%20Fly%20Speed :type Float%20%28double-precision%29))
  (Variables|/Script/Engine.CharacterMovementComponent|SetMaxFlySpeed (Variables|Character|GetCharacterMovement) New%20Fly%20Speed))