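; EnemyProjectile is a projectile actor fired in the game's enemy combat that damages the player on contact.
; On BeginPlay it multiplies its projectile movement velocity tenfold and destroys itself after a short lifetime.
; Its sphere overlap ignores other projectiles and both flyer enemy types, damages the player when hitting the HorrorEngineCharacter, and otherwise destroys itself on any other overlap.
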(event OnComponentBeginOverlap(Spherecol)
  (params (OverlappedComponent :type Primitive%20Component%20Object%20Reference) (OtherActor :type Actor%20Object%20Reference) (OtherComp :type Primitive%20Component%20Object%20Reference) (OtherBodyIndex :type Integer) (bFromSweep :type Boolean) (SweepResult :type Hit%20Result%20Structure%20%28by%20ref%29))
  (Utilities|Casting|CastToEnemyProjectile OtherActor
    (:CastFailed
      (Utilities|Casting|CastToBP_Flyer OtherActor
        (:CastFailed
          (Utilities|Casting|CastToBigFlyer OtherActor
            (:CastFailed
              (Utilities|Casting|CastToHorrorEngineCharacter OtherActor
                (:then
                  (bind _asmaster (CallFunction|GetPlayer))
                  (Default|GetDamage :self _asmaster :DamagePoint 1e+01)
                  (Actor|DestroyActor))
                (:CastFailed
                  (Actor|DestroyActor))))))))))

(event EventBeginPlay
  (bind _projectilemovement (Variables|Default|GetProjectileMovement))
  (Variables|/Script/Engine.MovementComponent|SetVelocity _projectilemovement (* (Variables|/Script/Engine.MovementComponent|GetVelocity _projectilemovement) "10.000000,10.000000,10.000000"))
  (Utilities|FlowControl|Delay 4.0)
  (Actor|DestroyActor))

(event EventTick
  (params (DeltaSeconds :type Float%20%28single-precision%29)))

(fn ConstructionScript)